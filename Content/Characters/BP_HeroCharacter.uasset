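; BP_HeroCharacter is a hero character with a right-mouse aim mode.
; Holding the button plays the Zoom timeline to drive spring arm length, and releasing it reverses the timeline.
; Each timeline update also applies the aiming flag to camera pawn-control rotation and controller yaw, and lowers walk speed while aiming.
; BeginPlay enables input from the first player controller.
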(event EventBeginPlay
  (Input|EnableInput (Game|GetPlayerController 0)))

(event EventTick
  (params (DeltaSeconds :type Float%20%28single-precision%29)))

(event Input|MouseEvents|RightMouseButton
  (params (Key :type Key%20Structure :default "None"))
  (:Pressed
    (Variables|Default|SetbIsAiming true)
    (bind _armlength (Timeline|Zoom Play)
      (:Update
        (Variables|/Script/Engine.SpringArmComponent|SetTargetArmLength (Variables|Default|GetSpringArm) _armlength)
        (Variables|/Script/Engine.CameraComponent|SetbUsePawnControlRotation (Variables|Default|GetCamera) (Variables|Default|GetbIsAiming))
        (Variables|Default|SetbUseControllerRotationYaw (Variables|Default|GetbIsAiming))
        (if (== (Variables|Default|GetbIsAiming) true)
          (Variables|/Script/Engine.CharacterMovementComponent|SetMaxWalkSpeed (Variables|Character|GetCharacterMovement) 3e+02)
          (else
            (Variables|/Script/Engine.CharacterMovementComponent|SetMaxWalkSpeed (Variables|Character|GetCharacterMovement) 6e+02))))))
  (:Released
    (Variables|Default|SetbIsAiming false)
    (Timeline|Zoom Reverse)))

(fn ConstructionScript)