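; BP_PrimitiveEnemy is a melee enemy character that spawns a BP_Sword on BeginPlay, attaches it to the right-hand socket and stores it as its equipped item.
; AttackInitiated hands off to InitiateAttack, which the author's note says runs through C++ to generalize the solution.
; InitiateAttackBP plays the given montage section on the mesh and calls CallOnAttackEnd whether it completes or is interrupted.
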(event Custom|AttackInitiated
  (Class|CharacterInterface|InitiateAttack) ; We call it through C++ to generalize solution. TODO: find cal PlayMontage with OnCompleted/OnInterrupted in c++
)

(event EventBeginPlay
  (bind _returnvalue (Game|SpawnActorfromClass "/Game/Models/Items/BP_Sword.BP_Sword_C" (Math|Conversions|ToTransform(Vector) (Transformation|GetActorLocation)) "Undefined" 0 0))
  (Class|Item|OnItemEquipped _returnvalue)
  (Transformation|AttachComponentToComponent _returnvalue (Variables|Character|GetMesh) "RightHandSocket" "SnapToTarget" "SnapToTarget" "KeepWorld" true)
  (Variables|Default|SetEquippedItem _returnvalue))

(event EventInitiateAttackBP
  (params (MontageToPlay :type Anim%20Montage%20Object%20Reference) (SectionName :type Name :default "None"))
  (Animation|Montage|PlayMontage (Variables|Character|GetMesh) MontageToPlay 1.0 0.0 SectionName
    (:OnCompleted
      _)
    (:OnInterrupted
      _))
  (Default|CallOnAttackEnd))

(fn ConstructionScript)